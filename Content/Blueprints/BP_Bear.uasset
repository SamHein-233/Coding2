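; BP_Bear is a collectible bear that the player character picks up by walking into its Sphere.
; The overlap adds the bear to the CollectedBears list in GM_Coding2's LevelSave, then calls LoadBears.
; LoadBears hides the bear, disables collision on its torso and legs, and triggers a game mode Checkpoint.
; That checkpoint takes its location from a BP_Flag's pole and its rotation and scale from the overlapping actor.
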(event OnComponentBeginOverlap(Sphere)
  (params (OverlappedComponent :type Primitive%20Component%20Object%20Reference) (OtherActor :type Actor%20Object%20Reference) (OtherComp :type Primitive%20Component%20Object%20Reference) (OtherBodyIndex :type Integer) (bFromSweep :type Boolean) (SweepResult :type Hit%20Result%20Structure%20%28by%20ref%29))
  (Utilities|Casting|CastToBP_ThirdPersonCharacter OtherActor)
  (bind _asgm_coding_2 (Utilities|Casting|CastToGM_Coding2 (Game|GetGameMode)))
  (Utilities|Array|AddUnique (Variables|/Game/Blueprints/SaveGames/SG_LevelSave.SG_LevelSave_C|GetCollectedBears (Variables|/Game/Blueprints/SaveGames/GM_Coding2.GM_Coding2_C|GetLevelSave _asgm_coding_2)) self)
  (CallFunction|LoadBears))

(event Custom|LoadBears
  (Rendering|SetVisibility (Variables|Default|GetDefaultSceneRoot) false true)
  (Collision|SetCollisionEnabled (Variables|Default|GetTorso) "NoCollision")
  (bind _returnvalue (Actor|GetActorOfClass "/Game/Blueprints/BP_Flag.BP_Flag_C"))
  (Default|Checkpoint (stale OnComponentBeginOverlap(Sphere) _asgm_coding_2) (Math|Transform|MakeTransform (+ (Transformation|GetWorldLocation (Variables|/Game/Blueprints/BP_Flag.BP_Flag_C|GetFlagPole _returnvalue)) "") (.rotation (Transformation|GetActorTransform (stale OnComponentBeginOverlap(Sphere) OtherActor))) (.scale (Transformation|GetActorTransform (stale OnComponentBeginOverlap(Sphere) OtherActor))))))

(event EventBeginPlay)

(event Collision|EventActorBeginOverlap
  (params (OtherActor :type Actor%20Object%20Reference)))

(event EventTick
  (params (DeltaSeconds :type Float%20%28single-precision%29)))

(fn ConstructionScript)