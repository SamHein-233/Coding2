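; SG_LevelSave is a level save asset that restores the state of collected coins and opened doors.
; It keeps both as arrays of object references, CollectedCoins and DoorsOpened, each with its own restore function.
; LoadCollectedCoins and DoorState loop over their array, skip invalid entries and call LoadCollectedState or LoadDoorState, so each object applies its own saved state.
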(fn LoadCollectedCoins
  (if (> (Utilities|Array|Length (Variables|Default|GetCollectedCoins)) 0)
    (for _array_element (Variables|Default|GetCollectedCoins)
      (Utilities|IsValid _array_element
        (:Is%20Valid
          (Default|LoadCollectedState _array_element))))))

(fn DoorState
  (if (> (Utilities|Array|Length (Variables|Default|GetDoorsOpened)) 0)
    (for _array_element (Variables|Default|GetDoorsOpened)
      (Utilities|IsValid _array_element
        (:Is%20Valid
          (Default|LoadDoorState _array_element))))))