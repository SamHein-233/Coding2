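; GM_Coding2 is a game mode that manages per-level saves, using the level name as the slot name.
; On BeginPlay it loads SG_LevelSave to restore coins, door state, bear collection and a non-zero player location's transform, or creates a fresh save if missing or invalid.
; Checkpoint stores the player transform and FinishedLevel clears it, both writing to the slot through SaveGame.
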(event Custom|SaveGame
  (bind _returnvalue (Game|GetCurrentLevelName true))
  (bind _returnvalue_2 (SaveGame|SaveGametoSlot (Variables|Default|GetLevelSave) _returnvalue))
  (if _returnvalue_2
    (Development|PrintString "Saved Level" true true "(R=0.013896,G=1.000000,B=0.000000,A=1.000000)")
    (else
      (Development|PrintString "Unable to save level" true true "(R=1.000000,G=0.000000,B=0.015610,A=1.000000)"))))

(event EventBeginPlay
  (Development|PrintString "Loaded into GM_Coding2 Game Mode")
  (bind _returnvalue (Game|GetCurrentLevelName true))
  (bind _returnvalue_2 (SaveGame|DoesSaveGameExist _returnvalue))
  (if _returnvalue_2
    (bind _returnvalue_3 (SaveGame|LoadGamefromSlot _returnvalue))
    (bind _assg_level_save (Utilities|Casting|CastToSG_LevelSave _returnvalue_3)
      (:then
        (bind _output_get (Variables|Default|SetLevelSave _assg_level_save))
        (Default|LoadCollectedCoins _output_get) ; Change the coins that have already been collected
        (Default|DoorState _output_get)
        (Default|CollectedBear _output_get)
        (if (not (Class|KismetMathLibrary|EqualExactlyVectorVector (.location (Variables|/Game/Blueprints/SaveGames/SG_LevelSave.SG_LevelSave_C|GetPlayerTransform (Variables|Default|GetLevelSave))) "0, 0, 0"))
          (Transformation|SetWorldTransform (Variables|/Script/Engine.Character|GetCapsuleComponent (Game|GetPlayerCharacter 0)) (Variables|/Game/Blueprints/SaveGames/SG_LevelSave.SG_LevelSave_C|GetPlayerTransform (Variables|Default|GetLevelSave)) false false)))
      (:CastFailed
        (SaveGame|DeleteGameinSlot _returnvalue)
        (bind _returnvalue_4 (SaveGame|CreateSaveGameObject "/Game/Blueprints/SaveGames/SG_LevelSave.SG_LevelSave_C" :!label _label))
        (Variables|Default|SetLevelSave _returnvalue_4)))
    (else
      (goto _label))))

(fn ConstructionScript)

(fn Checkpoint
  (params (PlayerTransform :type Transform))
  (Variables|/Game/Blueprints/SaveGames/SG_LevelSave.SG_LevelSave_C|SetPlayerTransform (Variables|Default|GetLevelSave) PlayerTransform)
  (CallFunction|SaveGame))

(fn FinishedLevel
  (Variables|/Game/Blueprints/SaveGames/SG_LevelSave.SG_LevelSave_C|SetPlayerTransform (Variables|Default|GetLevelSave) "")
  (CallFunction|SaveGame))