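; BP_CarTrigger is a trigger volume that celebrates a BP_ThirdPersonCharacter entering its box with effects and a car widget.
; On overlap, it activates the PSparksG sparks and plays the Victory sound at the box's relative, not world, location.
; After 2.5 seconds, it creates W_CarWidget for the controller matching that character's PlayerControllerID and adds it to that player's screen.
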(event OnComponentBeginOverlap(Box)
  (params (OverlappedComponent :type Primitive%20Component%20Object%20Reference) (OtherActor :type Actor%20Object%20Reference) (OtherComp :type Primitive%20Component%20Object%20Reference) (OtherBodyIndex :type Integer) (bFromSweep :type Boolean) (SweepResult :type Hit%20Result%20Structure%20%28by%20ref%29))
  (bind _asbp_third_person_character (Utilities|Casting|CastToBP_ThirdPersonCharacter OtherActor))
  (Components|Activation|Activate (Variables|Default|GetP_Sparks_G) true)
  (Audio|PlaySoundatLocation "/Game/Audio/GameDesign3/Victory.Victory" (Variables|/Script/Engine.SceneComponent|GetRelativeLocation (Variables|Default|GetBox)) "0, 0, 0" 1.0 1.0 0.0 0 0 0 0)
  (Utilities|FlowControl|Delay 2.5)
  (bind _returnvalue (UserInterface|CreateWidget "/Game/WidgetsUI/W_CarWidget.W_CarWidget_C" (Class|GameplayStatics|GetPlayerControllerfromID (Variables|/Game/ThirdPerson/Blueprints/BP_ThirdPersonCharacter.BP_ThirdPersonCharacter_C|GetPlayerControllerID _asbp_third_person_character))))
  (bind _output_get (Variables|Default|SetW_CarRef _returnvalue))
  (UserInterface|Viewport|AddtoPlayerScreen _output_get))

(event EventBeginPlay)

(event Collision|EventActorBeginOverlap
  (params (OtherActor :type Actor%20Object%20Reference)))

(event EventTick
  (params (DeltaSeconds :type Float%20%28single-precision%29)))

(fn ConstructionScript)