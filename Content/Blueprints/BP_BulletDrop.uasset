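; BP_BulletDrop is an actor that repeatedly fires a simulated bullet with gravity drop from its Arrow component, every 0.2 seconds.
; BulletDropCalculator approximates the arc with stepped line traces, lowering Z velocity each step, with SimFrequency setting step size and count.
; On the first hit it plays a sound, spawns a blood emitter and passes the impact data to the player character's BulletDrop.
; Predict-path and debug-draw nodes are left unconnected.
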(event Custom|BulletDropCalculator
  (Variables|Default|SetEnd (+ (Variables|Default|GetStart) (/ (Variables|Default|GetVelocity) (Math|Vector|MakeVector (Variables|Default|GetSimFrequency) 1.0 1.0))))
  (Utilities|FlowControl|ForLoopwithBreak 1 (Math|Float|Truncate (Variables|Default|GetSimFrequency)) :!label _label
    (:LoopBody
      (bind _returnvalue (Class|KismetSystemLibrary|LineTraceSinglebyProfile (Variables|Default|GetStart) (Variables|Default|GetEnd) "BlockAll" false 0 "None" true))
      (if _returnvalue
        (Audio|PlaySoundatLocation "/Game/Audio/HitSound.HitSound" (Variables|Default|GetEnd) "0, 0, 0" 1.0 1.0 0.0 0 0 0 0)
        (Effects|SpawnEmitteratLocation "/Game/Realistic_Starter_VFX_Pack_Vol2/Particles/Blood/P_Blood_Splat_Cone.P_Blood_Splat_Cone" (Variables|Default|GetEnd) "90.000000,0.000000,0.000000")
        (bind _asbp_third_person_character (Utilities|Casting|CastToBP_ThirdPersonCharacter (Game|GetPlayerCharacter 0)))
        (Default|BulletDrop _asbp_third_person_character (Variables|Default|GetEnd) (Variables|Default|GetVelocity) (Variables|Default|GetMaxSimTime))
        (goto _label Break)
        (else
          (Variables|Default|SetStart (Variables|Default|GetEnd))
          (Variables|Default|SetVelocity (+ (Variables|Default|GetVelocity) (Math|Vector|MakeVector 0.0 0.0 (/ -9.8e+02 (Math|Float|Square (Variables|Default|GetSimFrequency))))))
          (Variables|Default|SetEnd (+ (Variables|Default|GetStart) (/ (Variables|Default|GetVelocity) (Math|Vector|MakeVector (Variables|Default|GetSimFrequency) 1.0 1.0)))))))
    (:Completed
      (Variables|Default|SetStart (Transformation|GetWorldLocation (Variables|Default|GetArrow)))
      (Variables|Default|SetVelocity (Variables|Default|GetStartVelocity)))))

(event EventBeginPlay
  (Variables|Default|SetStart (Transformation|GetWorldLocation (Variables|Default|GetArrow)))
  (Utilities|FlowControl|Sequence :!label _label
    (:then_0
      (CallFunction|BulletDropCalculator)
      (Utilities|FlowControl|Delay 0.2)
      (goto _label))))

(fn ConstructionScript)