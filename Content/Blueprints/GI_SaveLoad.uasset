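; Save/load Blueprint for the player and per-level data, though every event is empty and all logic chains are disconnected.
; Those chains store stamina, transform and sprint/shoot flags in SG_Coding2, and SG_SaveLevel data in a slot named after the level.
; Load and create fallbacks, collected-object restore, deletion of both slots and debug prints are included.
; The load chain copies sprint/shoot flags from character to save, so these are never restored.
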(event Custom|SaveGame)

(event Custom|Save%20Level)

(event Custom|Load%20Level)

(event Custom|DeleteSaveData)

(event Custom|LoadGame)

(event Custom|Status)

(event EventInit)