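; BP_Weapon is a weapon actor meant to show a randomized weapon with type, element and damage range text.
; On BeginPlay it looks up a random DT_Weapons row, though the graph shows no use of that row and no call to RandomizeValue.
; RandomizeValue rolls min and max damage, then refreshes the text and sets the mesh, choosing its material by weapon type.
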(event Custom|SpawnWeapon
  (bind _outrownames (DataTable|GetDataTableRowNames "/Game/DataTables/DT_Weapons.DT_Weapons"))
  (Utilities|GetDataTableRow "/Game/DataTables/DT_Weapons.DT_Weapons" (.OutItem (Utilities|Array|Random _outrownames))))

(event Custom|RandomizeValue
  (bind _output_get (Variables|Default|SetMinDamage (+ (Variables|Default|GetMinDamage) (Math|Random|RandomInteger 2))))
  (Variables|Default|SetMaxDamage (+ _output_get (Math|Random|RandomIntegerinRange 1 4)))
  (CallFunction|UpdateText)
  (CallFunction|SetMesh))

(event Custom|UpdateText
  (Rendering|Components|TextRender|SetText (Variables|Default|GetTextWeaponType) (Utilities|Text|ToText(String) (Utilities|String|EnumtoString (Variables|Default|GetWeaponType))))
  (Rendering|Components|TextRender|SetText (Variables|Default|GetElementType) (Utilities|Text|ToText(String) (Utilities|String|EnumtoString (Variables|Default|GetElementalType))))
  (Rendering|Components|TextRender|SetText (Variables|Default|GetDamage) (Utilities|Text|ToText(String) (Utilities|String|Append (Utilities|String|ToString(Integer) (Variables|Default|GetMinDamage)) " - " (Utilities|String|ToString(Integer) (Variables|Default|GetMaxDamage))))))

(event Custom|SetMesh
  (bind _weaponbody (Variables|Default|GetWeaponBody))
  (Components|StaticMesh|SetStaticMesh _weaponbody (Variables|Default|GetWeaponMesh))
  (Rendering|Material|SetMaterial _weaponbody 0 (Utilities|Array|Get(acopy) (Variables|Default|GetWeaponMaterials) (Math|Conversions|ToInteger(Byte) (Variables|Default|GetWeaponType)))))

(event EventBeginPlay
  (CallFunction|SpawnWeapon))

(event Collision|EventActorBeginOverlap
  (params (OtherActor :type Actor%20Object%20Reference)))

(event EventTick
  (params (DeltaSeconds :type Float%20%28single-precision%29)))

(fn ConstructionScript)