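; Dialogue trigger actor that lets the third-person character step through lines from DT_Dialogue by pressing E.
; Overlapping its collision enables input and shows a talk prompt widget; leaving only disables input.
; Each press removes the prompt and writes the next row's text, emotion and image material into a dialogue widget created on BeginPlay.
; A resettable DoOnce gates adding that widget to the viewport; after the last row it closes and rewinds.
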(event OnComponentBeginOverlap(Collision)
  (params (OverlappedComponent :type Primitive%20Component%20Object%20Reference) (OtherActor :type Actor%20Object%20Reference) (OtherComp :type Primitive%20Component%20Object%20Reference) (OtherBodyIndex :type Integer) (bFromSweep :type Boolean) (SweepResult :type Hit%20Result%20Structure%20%28by%20ref%29))
  (Utilities|Casting|CastToBP_ThirdPersonCharacter OtherActor)
  (Input|EnableInput (Game|GetPlayerController 0))
  (bind _returnvalue (UserInterface|CreateWidget "/Game/DataTables/DialogueSystem/W_Talk.W_Talk_C"))
  (bind _output_get (Variables|Default|SetTalkRef _returnvalue))
  (UserInterface|Viewport|AddtoViewport _output_get 0))

(event OnComponentEndOverlap(Collision)
  (params (OverlappedComponent :type Primitive%20Component%20Object%20Reference) (OtherActor :type Actor%20Object%20Reference) (OtherComp :type Primitive%20Component%20Object%20Reference) (OtherBodyIndex :type Integer))
  (Utilities|Casting|CastToBP_ThirdPersonCharacter OtherActor)
  (Input|DisableInput (Game|GetPlayerController 0)))

(event Custom|NextLine
  (Utilities|FlowControl|Sequence
    (:then_0
      (Utilities|FlowControl|DoOnce false
        (:Completed
          (UserInterface|Viewport|AddtoViewport (Variables|Default|GetDialogueRef) 0))))
    (:then_1
      (bind _outrownames (DataTable|GetDataTableRowNames "/Game/DataTables/DialogueSystem/DT_Dialogue.DT_Dialogue"))
      (if (< (Variables|Default|GetRowIndex) (Utilities|Array|Length _outrownames))
        (bind _returnvalue (Utilities|GetDataTableRow "/Game/DataTables/DialogueSystem/DT_Dialogue.DT_Dialogue" (Utilities|Array|Get(acopy) _outrownames (Variables|Default|GetRowIndex)))
          (:then
            (Rendering|Components|TextRender|SetText (Variables|/Game/DataTables/DialogueSystem/W_DataTableDialogue.W_DataTableDialogue_C|GetDialogue (stale EventBeginPlay _returnvalue)) (.text _returnvalue))
            (Rendering|Components|TextRender|SetText (Variables|/Game/DataTables/DialogueSystem/W_DataTableDialogue.W_DataTableDialogue_C|GetEmotion (stale EventBeginPlay _returnvalue)) (Utilities|Text|ToText(String) (Utilities|String|EnumtoString (.emotion _returnvalue))))
            (Appearance|GetDynamicMaterial (Variables|/Game/DataTables/DialogueSystem/W_DataTableDialogue.W_DataTableDialogue_C|GetImage_48 (stale EventBeginPlay _returnvalue)) :!class /Script/UMG.Image)
            (Class|Image|SetBrushfromMaterial (Variables|/Game/DataTables/DialogueSystem/W_DataTableDialogue.W_DataTableDialogue_C|GetImage_48 (stale EventBeginPlay _returnvalue)) (.image _returnvalue))
            (Math|Integer|IncrementInt (Variables|Default|GetRowIndex))))
        (else
          (Widget|RemovefromParent (Variables|Default|GetDialogueRef))
          (CallFunction|ResetAddtoViewport)
          (Variables|Default|SetRowIndex 0))))))

(event Custom|ResetAddToViewport
  (Utilities|FlowControl|DoOnce false) ; enters at Reset
)

(event EventBeginPlay
  (bind _returnvalue (UserInterface|CreateWidget "/Game/DataTables/DialogueSystem/W_DataTableDialogue.W_DataTableDialogue_C"))
  (Variables|Default|SetDialogueRef _returnvalue))

(event Input|KeyboardEvents|E
  (params (Key :type Key%20Structure :default "None"))
  (:Pressed
    (Widget|RemovefromParent (Variables|Default|GetTalkRef))
    (CallFunction|NextLine)))

(fn ConstructionScript)