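; BP_WeaponSpawner spawns a random weapon when the third-person character enters its trigger sphere.
; Each overlap picks a random DT_Weapons row and spawns a BP_Weapon at the sphere's location, with no guard against repeat spawns.
; It copies the row's weapon type, element, base damage (as minimum damage), mesh and material onto the weapon, then calls RandomizeValue on it.
; Leftover text-setting nodes for type, element and damage never run.
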(event OnComponentBeginOverlap(Sphere1)
  (params (OverlappedComponent :type Primitive%20Component%20Object%20Reference) (OtherActor :type Actor%20Object%20Reference) (OtherComp :type Primitive%20Component%20Object%20Reference) (OtherBodyIndex :type Integer) (bFromSweep :type Boolean) (SweepResult :type Hit%20Result%20Structure%20%28by%20ref%29))
  (Utilities|Casting|CastToBP_ThirdPersonCharacter OtherActor)
  (CallFunction|SpawnWeapon))

(event Custom|SpawnWeapon
  (bind _outrownames (DataTable|GetDataTableRowNames "/Game/DataTables/DT_Weapons.DT_Weapons"))
  (bind _returnvalue (Utilities|GetDataTableRow "/Game/DataTables/DT_Weapons.DT_Weapons" (.OutItem (Utilities|Array|Random _outrownames)))
    (:then
      (bind _returnvalue_2 (Game|SpawnActorfromClass "/Game/DataTables/BP_Weapon.BP_Weapon_C" (Math|Transform|MakeTransform (Transformation|GetWorldLocation (Variables|Default|GetSphere1)) "0, 0, 0" "1.000000,1.000000,1.000000") "Undefined" "MultiplyWithRoot" 0 0))
      (Variables|/Game/DataTables/BP_Weapon.BP_Weapon_C|SetWeaponType _returnvalue_2 (.weapontype _returnvalue))
      (Variables|/Game/DataTables/BP_Weapon.BP_Weapon_C|SetElementalType _returnvalue_2 (.elementaltype _returnvalue))
      (Variables|/Game/DataTables/BP_Weapon.BP_Weapon_C|SetMinDamage _returnvalue_2 (.basedamage _returnvalue))
      (Variables|/Game/DataTables/BP_Weapon.BP_Weapon_C|SetWeaponMesh _returnvalue_2 (.staticmesh _returnvalue))
      (Variables|/Game/DataTables/BP_Weapon.BP_Weapon_C|SetWeaponMaterial _returnvalue_2 (.material _returnvalue))
      (Default|RandomizeValue _returnvalue_2))))

(event EventBeginPlay)

(event Collision|EventActorBeginOverlap
  (params (OtherActor :type Actor%20Object%20Reference)))

(event EventTick
  (params (DeltaSeconds :type Float%20%28single-precision%29)))

(fn ConstructionScript)